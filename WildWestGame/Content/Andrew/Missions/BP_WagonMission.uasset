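; BP_WagonMission is a wagon mission Blueprint that tracks the wagon's health and a countdown timer.
; BeginPlay sets both from their base values.
; Tick uses a DoOnce gate, reset after a one-second Delay, to reduce WagonTime by one roughly every second.
; The graph has no stop condition for the timer and does not use WagonHealth after initialization.
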(event `self.ReceiveBeginPlay`
  (set `self.WagonHealth` (`self.WagonBaseHealth`))
  (set `self.WagonTime` (`self.WagonBaseTime`)))

(event `self.ReceiveTick`
  (params (DeltaSeconds :type "Float (single-precision)"))
  (if true
    (`/Engine/EditorBlueprintResources/StandardMacros.DoOnce` false :!label _label
      (:`Completed`
        (`KismetSystemLibrary.Delay` 1.0)
        (set `self.WagonTime` (- (`self.WagonTime`) 1.0))
        (goto _label :!via `Reset`)))))

(fn `UserConstructionScript`)